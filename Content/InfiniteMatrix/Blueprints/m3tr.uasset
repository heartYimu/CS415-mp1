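; Hazard actor with a donut guardian mesh that hurts the player on contact and can be destroyed by BP_shut for score.
; Mesh hits call Hurt and ChangeDead, then either show restart if dead or deduct score, shove the player along X and self-destroy.
; Box overlap with BP_shut destroys both and adds score to the first BP_Player found.
; It expires on a lifespan, or earlier when off-screen after a short delay.
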(event `self.ReceiveBeginPlay`
  (`self.SetLifeSpan` 10.0)
  (`KismetSystemLibrary.Delay` 2.0)
  (set `self.Render?` true))

(event `self.ReceiveTick`
  (params (DeltaSeconds :type "Float (single-precision)"))
  (if (`self.Render?`)
    (if (not (`self.WasRecentlyRendered` 1.0))
      (`self.K2_DestroyActor`))))

(event `self.donut_guardian_0409163206_texture_fbx.OnComponentHit`
  (params (HitComponent :type "PrimitiveComponent Object Reference") (OtherActor :type "Actor Object Reference") (OtherComp :type "PrimitiveComponent Object Reference") (NormalImpulse :type "Vector Structure") (Hit :type "HitResult Structure (by ref)"))
  (bind _asbp_player (cast `/Game/InfiniteMatrix/Blueprints/BP_Player` OtherActor))
  (`/Game/InfiniteMatrix/Blueprints/BP_Player.Hurt` _asbp_player)
  (`/Game/InfiniteMatrix/Blueprints/BP_Player.ChangeDead` _asbp_player)
  (if (`/Game/InfiniteMatrix/Blueprints/BP_Player.IsDead` _asbp_player)
    (if (not (`/Game/InfiniteMatrix/Blueprints/BP_Player.restart?` _asbp_player))
      (`/Game/InfiniteMatrix/Blueprints/BP_Player.DisplayRestart` _asbp_player)
      (`self.K2_DestroyActor`)
      (set `/Game/InfiniteMatrix/Blueprints/BP_Player.IsDead` true _asbp_player)
      (set `/Game/InfiniteMatrix/Blueprints/BP_Player.restart?` true _asbp_player))
    (else
      (`/Game/InfiniteMatrix/Blueprints/BP_Player.Minus score` _asbp_player)
      (`self.K2_AddActorWorldOffset` _asbp_player (200.0 0.0 0.0) false false)
      (`self.K2_DestroyActor`))))

(event `self.Box.OnComponentHit`
  (params (HitComponent :type "PrimitiveComponent Object Reference") (OtherActor :type "Actor Object Reference") (OtherComp :type "PrimitiveComponent Object Reference") (NormalImpulse :type "Vector Structure") (Hit :type "HitResult Structure (by ref)")))

(event `self.Box.OnComponentBeginOverlap`
  (params (OverlappedComponent :type "PrimitiveComponent Object Reference") (OtherActor :type "Actor Object Reference") (OtherComp :type "PrimitiveComponent Object Reference") (OtherBodyIndex :type Integer) (bFromSweep :type Boolean) (SweepResult :type "HitResult Structure (by ref)"))
  (bind _asbp_shut (cast `/Game/InfiniteMatrix/Blueprints/BP_shut` OtherActor))
  (`self.K2_DestroyActor` _asbp_shut)
  (`self.K2_DestroyActor`)
  (bind _outactors (`GameplayStatics.GetAllActorsOfClass` "/Game/InfiniteMatrix/Blueprints/BP_Player.BP_Player_C"))
  (`/Game/InfiniteMatrix/Blueprints/BP_Player.ADD score` (`|GetArrayItem` _outactors)))

(fn `UserConstructionScript`)