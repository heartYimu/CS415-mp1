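; Tunnel segment for an endless runner, with a rotating holed wall that the player must pass.
; BeginPlay spawns an M3tr and, half the time, a health pack at random points within the actor's bounds.
; Passing the trigger adds score, has TunnelSpawner spawn another tunnel and destroys this one.
; Wall hits hurt the player, then either show restart or deduct score and nudge them; RandomizeWall, uncalled here, randomizes mesh and roll.
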(event `self.ReceiveBeginPlay`
  (`self.Spawn m3tr`)
  (`self.Hasmedbag?`)
  (if (`self.HasHealthPack`)
    (`self.Spawn medbag`)
    (set `self.HasHealthPack` false)))

(event `self.ReceiveTick`
  (params (DeltaSeconds :type "Float (single-precision)"))
  (`SceneComponent.K2_AddLocalRotation` (`self.WallMesh`) (`KismetMathLibrary.MakeRotator` (* DeltaSeconds (`self.RotateSpeed`))) false false))

(event `self.TriggerZone.OnComponentBeginOverlap`
  (params (OverlappedComponent :type "PrimitiveComponent Object Reference") (OtherActor :type "Actor Object Reference") (OtherComp :type "PrimitiveComponent Object Reference") (OtherBodyIndex :type Integer) (bFromSweep :type Boolean) (SweepResult :type "HitResult Structure (by ref)"))
  (bind _asbp_player (cast `/Game/InfiniteMatrix/Blueprints/BP_Player` OtherActor))
  (`/Game/InfiniteMatrix/Blueprints/BP_Player.ADD score` _asbp_player)
  (`/Game/InfiniteMatrix/Blueprints/BP_TunnelSpawner.SpawnTunnelAtSpawnPoint` (`self.TunnelSpawner`))
  (`self.K2_DestroyActor`))

(event `self.WallMesh.OnComponentHit`
  (params (HitComponent :type "PrimitiveComponent Object Reference") (OtherActor :type "Actor Object Reference") (OtherComp :type "PrimitiveComponent Object Reference") (NormalImpulse :type "Vector Structure") (Hit :type "HitResult Structure (by ref)"))
  (bind _asbp_player (cast `/Game/InfiniteMatrix/Blueprints/BP_Player` OtherActor))
  (`/Game/InfiniteMatrix/Blueprints/BP_Player.Hurt` _asbp_player)
  (`/Game/InfiniteMatrix/Blueprints/BP_Player.ChangeDead` _asbp_player)
  (if (`/Game/InfiniteMatrix/Blueprints/BP_Player.IsDead` _asbp_player)
    (if (not (`/Game/InfiniteMatrix/Blueprints/BP_Player.restart?` _asbp_player))
      (`/Game/InfiniteMatrix/Blueprints/BP_Player.DisplayRestart` _asbp_player)
      (set `/Game/InfiniteMatrix/Blueprints/BP_Player.restart?` true _asbp_player))
    (else
      (`/Game/InfiniteMatrix/Blueprints/BP_Player.Minus score` _asbp_player)
      (`self.K2_AddActorWorldOffset` _asbp_player (100.0 0.0 0.0) false false))))

(fn `Hasmedbag?`
  (set `self.HasHealthPack` (<= (`KismetMathLibrary.RandomFloatInRange` 0.0 1.0) 0.5)))

(fn `RandomizeWall`
  (`StaticMeshComponent.SetStaticMesh` (`self.WallMesh`) (select `int` (`KismetMathLibrary.RandomIntegerInRange` 0 3) :`0` "/Game/InfiniteMatrix/Meshes/SM_Hole_01.SM_Hole_01" :`1` "/Game/InfiniteMatrix/Meshes/SM_Hole_02.SM_Hole_02" :`2` "/Game/InfiniteMatrix/Meshes/SM_Hole_03.SM_Hole_03" :`3` "/Game/InfiniteMatrix/Meshes/SM_Hole_04.SM_Hole_04" :!type "StaticMesh Object Reference"))
  (`SceneComponent.K2_AddLocalRotation` (`self.WallMesh`) (`KismetMathLibrary.MakeRotator` (`KismetMathLibrary.RandomFloatInRange` 0.0 360.0)) false false))

(fn `Spawn m3tr`
  (bind (_origin _boxextent) (`self.GetActorBounds` false))
  (bind _x (.x _boxextent))
  (bind _y (.y _boxextent))
  (bind _z (.z _boxextent))
  (`|SpawnActorFromClass` "/Game/InfiniteMatrix/Blueprints/m3tr.m3tr_C" (`KismetMathLibrary.Conv_VectorToTransform` (`KismetMathLibrary.MakeVector` (+ (.x _origin) (`KismetMathLibrary.RandomFloatInRange` (* _x -0.4) (* _x 0.4))) (+ (.y _origin) (`KismetMathLibrary.RandomFloatInRange` (* _y -0.4) (* _y 0.4))) (+ (.z _origin) (`KismetMathLibrary.RandomFloatInRange` (* _z -0.4) (* _z 0.4))))) "Undefined" "MultiplyWithRoot" null null))

(fn `Spawn medbag`
  (bind (_origin _boxextent) (`self.GetActorBounds` false))
  (bind _x (.x _boxextent))
  (bind _y (.y _boxextent))
  (bind _z (.z _boxextent))
  (`|SpawnActorFromClass` "/Game/InfiniteMatrix/Blueprints/BP_HealthPack.BP_HealthPack_C" (`KismetMathLibrary.Conv_VectorToTransform` (`KismetMathLibrary.MakeVector` (+ (.x _origin) (`KismetMathLibrary.RandomFloatInRange` (* _x -0.4) (* _x 0.4))) (+ (.y _origin) (`KismetMathLibrary.RandomFloatInRange` (* _y -0.4) (* _y 0.4))) (+ (.z _origin) (`KismetMathLibrary.RandomFloatInRange` (* _z -0.4) (* _z 0.4))))) "Undefined" "MultiplyWithRoot" null null))

(fn `UserConstructionScript`)